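; Sample Dolby.io conference actor that drives the debug status and connect menu widgets for a voice conference.
; BeginPlay creates both widgets and enables input so the C key reveals the initially hidden menu; EndPlay removes them.
; Device events refresh the input and output combo boxes.
; Status changes update the debug text and toggle menu controls by matching a Connected or Disconnected prefix, with disconnection also clearing mute flags; the token refresh handler is empty.
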(event `self.ReceiveBeginPlay`
  ;[1 1 1] Create widgets
  (bind _returnvalue (`|CreateWidget` "/Cppsdk/DolbyIoSampleDebugInfo.DolbyIoSampleDebugInfo_C"))
  (bind _output_get (set `self.Debug Info Ref` _returnvalue))
  (`Widget.SetVisibility` _output_get "Visible")
  (`UserWidget.AddToViewport` _output_get 0)
  (set `/Cppsdk/DolbyIoSampleDebugInfo.Status` (`self.Status`) _output_get)
  (bind _returnvalue_2 (`|CreateWidget` "/Cppsdk/DolbyIoSampleConnectMenu.DolbyIoSampleConnectMenu_C"))
  (bind _output_get_2 (set `self.Connect Menu Ref` _returnvalue_2))
  (`Widget.SetVisibility` _output_get_2 "Hidden")
  (`UserWidget.AddToViewport` _output_get_2 0)
  ;[1 1 1] Bind key to show menu
  (`self.EnableInput` (`GameplayStatics.GetPlayerController` 0)))

(event `Key|C`
  (params (Key :type "Key Structure"))
  ;[1 1 1] Bind key to show menu
  (:`Pressed`
    (`Widget.SetVisibility` (`self.Connect Menu Ref`) "Visible")))

(event `self.ReceiveEndPlay`
  (params (EndPlayReason :type "EEndPlayReason Enum" :default "Destroyed"))
  ;[1 1 1] Remove widgets
  (`Widget.RemoveFromParent` (`self.Connect Menu Ref`))
  (`Widget.RemoveFromParent` (`self.Debug Info Ref`)))

(event `self.OnNewListOfInputDevices`
  (bind _inputdevicecombobox (`/Cppsdk/DolbyIoSampleConnectMenu.InputDeviceComboBox` (`self.Connect Menu Ref`)))
  ;[1 1 1] Device list handlers
  (`ComboBoxString.ClearOptions` _inputdevicecombobox)
  (for _array_element (`self.InputDevices`)
    (`ComboBoxString.AddOption` _inputdevicecombobox (`KismetTextLibrary.Conv_TextToString` _array_element))
    (`ComboBoxString.SetSelectedOption` _inputdevicecombobox (`KismetTextLibrary.Conv_TextToString` (`self.CurrentInputDevice`)))))

(event `self.OnNewListOfOutputDevices`
  (bind _outputdevicecombobox (`/Cppsdk/DolbyIoSampleConnectMenu.OutputDeviceComboBox` (`self.Connect Menu Ref`)))
  ;[1 1 1] Device list handlers
  (`ComboBoxString.ClearOptions` _outputdevicecombobox)
  (for _array_element (`self.OutputDevices`)
    (`ComboBoxString.AddOption` _outputdevicecombobox (`KismetTextLibrary.Conv_TextToString` _array_element))
    (`ComboBoxString.SetSelectedOption` _outputdevicecombobox (`KismetTextLibrary.Conv_TextToString` (`self.CurrentOutputDevice`)))))

(event `self.OnInputDeviceChanged`
  ;[1 1 1] Device changed handlers
  (`ComboBoxString.SetSelectedOption` (`/Cppsdk/DolbyIoSampleConnectMenu.InputDeviceComboBox` (`self.Connect Menu Ref`)) (`KismetTextLibrary.Conv_TextToString` (`self.CurrentInputDevice`))))

(event `self.OnOutputDeviceChanged`
  ;[1 1 1] Device changed handlers
  (`ComboBoxString.SetSelectedOption` (`/Cppsdk/DolbyIoSampleConnectMenu.OutputDeviceComboBox` (`self.Connect Menu Ref`)) (`KismetTextLibrary.Conv_TextToString` (`self.CurrentOutputDevice`))))

(event `self.OnStatusChanged`
  (bind _connect_menu_ref (`self.Connect Menu Ref`))
  (bind _connect_menu_ref_2 (`self.Connect Menu Ref`))
  ;[1 1 1] Status changed handler
  (bind _output_get (set `/Cppsdk/DolbyIoSampleDebugInfo.Status` (`self.Status`) (`self.Debug Info Ref`)))
  (if (`KismetStringLibrary.StartsWith` _output_get "Connected")
    (`Widget.SetIsEnabled` (`/Cppsdk/DolbyIoSampleConnectMenu.ConnectBtn` _connect_menu_ref_2) false)
    (`Widget.SetIsEnabled` (`/Cppsdk/DolbyIoSampleConnectMenu.DisconnectBtn` _connect_menu_ref_2) true)
    (`Widget.SetIsEnabled` (`/Cppsdk/DolbyIoSampleConnectMenu.InputMuteCheckBox` _connect_menu_ref_2) true)
    (`Widget.SetIsEnabled` (`/Cppsdk/DolbyIoSampleConnectMenu.OutputMuteCheckBox` _connect_menu_ref_2) true)
    (`Widget.SetIsEnabled` (`/Cppsdk/DolbyIoSampleConnectMenu.InputDeviceComboBox` _connect_menu_ref_2) true)
    (`Widget.SetIsEnabled` (`/Cppsdk/DolbyIoSampleConnectMenu.OutputDeviceComboBox` _connect_menu_ref_2) true)
    (elif (`KismetStringLibrary.StartsWith` _output_get "Disconnected")
      (`Widget.SetIsEnabled` (`/Cppsdk/DolbyIoSampleConnectMenu.ConnectBtn` _connect_menu_ref) true)
      (`Widget.SetIsEnabled` (`/Cppsdk/DolbyIoSampleConnectMenu.DisconnectBtn` _connect_menu_ref) false)
      (`Widget.SetIsEnabled` (`/Cppsdk/DolbyIoSampleConnectMenu.InputMuteCheckBox` _connect_menu_ref) false)
      (`Widget.SetIsEnabled` (`/Cppsdk/DolbyIoSampleConnectMenu.OutputMuteCheckBox` _connect_menu_ref) false)
      (`Widget.SetIsEnabled` (`/Cppsdk/DolbyIoSampleConnectMenu.InputDeviceComboBox` _connect_menu_ref) false)
      (`Widget.SetIsEnabled` (`/Cppsdk/DolbyIoSampleConnectMenu.OutputDeviceComboBox` _connect_menu_ref) false)
      (set `self.bIsInputMuted` false)
      (set `self.bIsOutputMuted` false))))

(event `self.OnRefreshTokenNeeded`
  ;[1 1 1] Refresh token handler
)

(fn `UserConstructionScript`)