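; Actor that spawns an in-world video plane for each non-screenshare Dolby.io video track.
; On track added, it spawns a BP_DolbyIOGenericVideoPlane, binds its material to the track ID and stores it in a map.
; Planes form a row along world Y from the spawner's location, spaced by plane scale.
; On track removed, it destroys that plane without reclaiming its slot in the row.
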(event `self.ReceiveBeginPlay`
  (set `self.Next Plane Location` (`self.K2_GetActorLocation`)))

(event `self.DolbyIOObserver.OnVideoTrackAdded`
  (params (VideoTrack :type "DolbyIOVideoTrack Structure (by ref)"))
  (bind (_trackid _participantid _bisscreenshare) (break `DolbyIOVideoTrack` VideoTrack))
  (bind (_next_plane_location_x _next_plane_location_y _next_plane_location_z) (`KismetMathLibrary.BreakVector` (`self.Next Plane Location`)))
  (bind _plane_scale_x (`KismetMathLibrary.BreakVector` (`self.Plane Scale`)))
  (if (not _bisscreenshare)
    (bind _returnvalue (`|SpawnActorFromClass` "/DolbyIO/BP_DolbyIOGenericVideoPlane.BP_DolbyIOGenericVideoPlane_C" (`KismetMathLibrary.MakeTransform` (`self.Next Plane Location`) (`self.Plane Rotation`) (`self.Plane Scale`)) "Undefined" "OverrideRootScale" null null))
    (`DolbyIOBlueprintFunctionLibrary.BindMaterial` (`/DolbyIO/BP_DolbyIOGenericVideoPlane.Video Material` _returnvalue) _trackid)
    (`BlueprintMapLibrary.Map_Add` (`self.Video Planes`) _trackid _returnvalue)
    (set `self.Next Plane Location` (`KismetMathLibrary.MakeVector` _next_plane_location_x (+ _next_plane_location_y (* (+ _plane_scale_x 0.1) 100.0)) _next_plane_location_z))))

(event `self.DolbyIOObserver.OnVideoTrackRemoved`
  (params (VideoTrack :type "DolbyIOVideoTrack Structure (by ref)"))
  (bind (_trackid _participantid _bisscreenshare) (break `DolbyIOVideoTrack` VideoTrack))
  (if (not _bisscreenshare)
    (`self.K2_DestroyActor` (`BlueprintMapLibrary.Map_Find` (`self.Video Planes`) _trackid))
    (`BlueprintMapLibrary.Map_Remove` (`self.Video Planes`) _trackid)))

(fn `UserConstructionScript`)