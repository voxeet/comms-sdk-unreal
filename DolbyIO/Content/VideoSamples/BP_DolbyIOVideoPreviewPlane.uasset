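; Preview plane actor that displays Dolby.io video on a static mesh.
; The construction script creates a dynamic instance of M_DolbyIOVideo and applies it to the mesh.
; DolbyIOObserver's video enabled and disabled events bind or unbind that material to the track ID, with no filtering, and show or hide the mesh.
; The mesh is hidden at BeginPlay.
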(event `self.DolbyIOObserver.OnVideoEnabled`
  (params (VideoTrackID :type String))
  (`DolbyIOBlueprintFunctionLibrary.BindMaterial` (`self.Video Material`) VideoTrackID)
  (`SceneComponent.SetVisibility` (`self.StaticMeshComponent`) true false))

(event `self.DolbyIOObserver.OnVideoDisabled`
  (params (VideoTrackID :type String))
  (`DolbyIOBlueprintFunctionLibrary.UnbindMaterial` (`self.Video Material`) VideoTrackID)
  (`SceneComponent.SetVisibility` (`self.StaticMeshComponent`) false false :!label _label))

(event `self.ReceiveBeginPlay`
  (goto _label))

(fn `UserConstructionScript`
  (bind _returnvalue (`KismetMaterialLibrary.CreateDynamicMaterialInstance` "/DolbyIO/VideoSamples/M_DolbyIOVideo.M_DolbyIOVideo"))
  (bind _output_get (set `self.Video Material` _returnvalue))
  (`PrimitiveComponent.SetMaterial` (`self.StaticMeshComponent`) 0 _output_get))