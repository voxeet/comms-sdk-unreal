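; Generic video plane for Dolby.io video samples, meant to show a video track on a static mesh.
; The construction script creates a dynamic instance of M_DolbyIOVideo, stores it as VideoMaterial and applies it to the mesh.
; DolbyIOObserver track added and removed events are empty stubs.
; BindMaterial and UnbindMaterial calls are present but unconnected, so no track reaches the material as it stands.
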(event `self.DolbyIOObserver.OnVideoTrackAdded`
  (params (VideoTrack :type "DolbyIOVideoTrack Structure (by ref)")))

(event `self.DolbyIOObserver.OnVideoTrackRemoved`
  (params (VideoTrack :type "DolbyIOVideoTrack Structure (by ref)")))

(fn `UserConstructionScript`
  (bind _returnvalue (`KismetMaterialLibrary.CreateDynamicMaterialInstance` "/DolbyIO/VideoSamples/M_DolbyIOVideo.M_DolbyIOVideo"))
  (bind _output_get (set `self.Video Material` _returnvalue))
  (`PrimitiveComponent.SetMaterial` (`self.StaticMeshComponent`) 0 _output_get))