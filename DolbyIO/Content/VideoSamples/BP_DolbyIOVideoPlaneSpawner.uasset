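; Sample spawner actor that shows each remote Dolby.io camera track on its own video plane in the level.
; When a track is added, it spawns a generic video plane, binds its material to the track and stores it by track ID.
; Planes line up along world Y from the spawner's location, spaced by plane scale.
; Removed tracks destroy their plane, but the next spawn position never moves back.
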(event `self.ReceiveBeginPlay`
  (set `self.Next Plane Location` (`self.K2_GetActorLocation`)))

(event `self.DolbyIOObserver.OnRemoteCameraTrackAdded`
  (params (TrackID :type String) (ParticipantID :type String))
  (bind (_next_plane_location_x _next_plane_location_y _next_plane_location_z) (`KismetMathLibrary.BreakVector` (`self.Next Plane Location`)))
  (bind _plane_scale_x (`KismetMathLibrary.BreakVector` (`self.Plane Scale`)))
  (bind _returnvalue (`|SpawnActorFromClass` "/DolbyIO/VideoSamples/BP_DolbyIOGenericVideoPlane.BP_DolbyIOGenericVideoPlane_C" (`KismetMathLibrary.MakeTransform` (`self.Next Plane Location`) (`self.Plane Rotation`) (`self.Plane Scale`)) "Undefined" "OverrideRootScale" null null))
  (`DolbyIOBlueprintFunctionLibrary.BindMaterial` (`/DolbyIO/VideoSamples/BP_DolbyIOGenericVideoPlane.Video Material` _returnvalue) TrackID)
  (`BlueprintMapLibrary.Map_Add` (`self.Video Planes`) TrackID _returnvalue)
  (set `self.Next Plane Location` (`KismetMathLibrary.MakeVector` _next_plane_location_x (+ _next_plane_location_y (* (+ _plane_scale_x 0.1) 100.0)) _next_plane_location_z)))

(event `self.DolbyIOObserver.OnRemoteCameraTrackRemoved`
  (params (TrackID :type String) (ParticipantID :type String))
  (`self.K2_DestroyActor` (`BlueprintMapLibrary.Map_Find` (`self.Video Planes`) TrackID))
  (`BlueprintMapLibrary.Map_Remove` (`self.Video Planes`) TrackID))

(fn `UserConstructionScript`)