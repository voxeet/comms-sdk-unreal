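; Screen-share display plane that shows Dolby.io screenshare video on its static mesh.
; The construction script creates a dynamic instance of the Dolby.io video material and applies it to the mesh.
; Dolby.io observer events bind that material to any added screenshare track and unbind it when the track is removed, ignoring non-screenshare tracks.
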(event `self.DolbyIOObserver.OnVideoTrackAdded`
  (params (VideoTrack :type "DolbyIOVideoTrack Structure (by ref)"))
  (bind (_trackid _participantid _bisscreenshare) (break `DolbyIOVideoTrack` VideoTrack))
  (if _bisscreenshare
    (`DolbyIOBlueprintFunctionLibrary.BindMaterial` (`self.Video Material`) _trackid)))

(event `self.DolbyIOObserver.OnVideoTrackRemoved`
  (params (VideoTrack :type "DolbyIOVideoTrack Structure (by ref)"))
  (bind (_trackid _participantid _bisscreenshare) (break `DolbyIOVideoTrack` VideoTrack))
  (if _bisscreenshare
    (`DolbyIOBlueprintFunctionLibrary.UnbindMaterial` (`self.Video Material`) _trackid)))

(fn `UserConstructionScript`
  (bind _returnvalue (`KismetMaterialLibrary.CreateDynamicMaterialInstance` "/DolbyIO/M_DolbyIOVideo.M_DolbyIOVideo"))
  (bind _output_get (set `self.Video Material` _returnvalue))
  (`PrimitiveComponent.SetMaterial` (`self.StaticMeshComponent`) 0 _output_get))