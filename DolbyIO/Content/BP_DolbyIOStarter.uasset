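; BP_DolbyIOStarter is an actor that starts Dolby.io voice conferencing and hosts a hidden sample menu, revealed with the M key.
; When the Dolby.io observer needs a token, it fetches one from the app key and secret if none is set, then initializes the SDK with it.
; After initialization, or on C, it joins a demo or configured spatial-audio conference; Ctrl+C disconnects.
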(event `self.ReceiveBeginPlay`
  (`self.EnableInput` (`GameplayStatics.GetPlayerController` 0))
  (bind _returnvalue (`|CreateWidget` "/DolbyIO/W_DolbyIOSampleMenu.W_DolbyIOSampleMenu_C"))
  (bind _output_get (set `self.Menu` _returnvalue))
  (`UserWidget.AddToViewport` _output_get 0)
  (`Widget.SetVisibility` _output_get "Hidden"))

(event `Key|M`
  (params (Key :type "Key Structure"))
  (:`Pressed`
    (`Widget.SetVisibility` (stale `self.ReceiveBeginPlay` _output_get) "Visible")))

(event `self.DolbyIOObserver.OnTokenNeeded`
  (if (`KismetStringLibrary.IsEmpty` (`self.Token`))
    (bind _token (`GetDolbyIOToken.GetDolbyIOToken` (`self.App Key`) (`self.App Secret`))
      (:`TokenObtained`
        (set `self.Token` _token))))
  (`DolbyIOSetToken.DolbyIOSetToken` (`self.Token`)
    (:`OnInitialized`
      (if (`self.bIsDemo`) :!label _label
        (`DolbyIODemoConference.DolbyIODemoConference`)
        (else
          (`DolbyIOConnect.DolbyIOConnect` (`self.Conference Name`) (`self.User Name`) "" "" (`self.Connection Mode`) (`self.Spatial Audio Style`)))))))

(event `Key|C`
  (params (Key :type "Key Structure"))
  (:`Pressed`
    (goto _label)))

(event `Key|Ctrl+C`
  (params (Key :type "Key Structure"))
  (:`Pressed`
    (`DolbyIODisconnect.DolbyIODisconnect`)))

(fn `UserConstructionScript`)